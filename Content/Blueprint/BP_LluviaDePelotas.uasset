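; BP_LluviaDePelotas is a moving spawner that creates a rain of BP_Pelota balls along a circular path.
; Each Tick advances Angulo by Velocidad and uses sine and cosine to sweep the actor horizontally around Centro at distance Radio.
; A Delay scaled from DeltaSeconds by DelayTime throttles spawning at the actor's current transform, so the interval depends on frame time.
; The CantidadPelotas variable is unused.
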(event `self.ReceiveTick`
  (params (DeltaSeconds :type "Float (single-precision)"))
  (bind (_centro_x _centro_y _centro_z) (`KismetMathLibrary.BreakVector` (`self.Centro`)))
  (set `self.Angulo` (+ (`self.Angulo`) (* DeltaSeconds (`self.Velocidad`))))
  (`self.K2_SetActorLocation` (`KismetMathLibrary.MakeVector` (+ (* (`KismetMathLibrary.Cos` (`self.Angulo`)) (`self.Radio`)) _centro_x) (+ _centro_y (* (`KismetMathLibrary.Sin` (`self.Angulo`)) (`self.Radio`))) _centro_z) true)
  (`KismetSystemLibrary.Delay` (* DeltaSeconds (`self.DelayTime`)))
  (`|SpawnActorFromClass` "/Game/Blueprint/BP_Pelota.BP_Pelota_C" (`self.GetTransform`) "Undefined" "MultiplyWithRoot" null null))

(fn `UserConstructionScript`)