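; BP_Ventilador is a fan actor that spins continuously at a slow, medium or fast preset.
; On BeginPlay, the Velocidad selection picks the matching delay time.
; A self-looping Delay then applies a fixed IntervaloGiro local rotation step on one axis each cycle, so speed comes from the wait between steps rather than from Tick.
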(event `self.ReceiveBeginPlay`
  (switch `/Game/Blueprint/EN_Velocidades` (`self.Velocidad`)
    (:`NewEnumerator0`
      (set `self.Vel` (`self.VelocidadLento`)))
    (:`NewEnumerator1`
      (set `self.Vel` (`self.VelocidadMedia`)))
    (:`NewEnumerator2`
      (set `self.Vel` (`self.VelocidadRapida`))))
  (`KismetSystemLibrary.Delay` (`self.Vel`) :!label _label)
  (set `self.VelocidadRotacion` (`KismetMathLibrary.MakeRotator` 0.0 (`self.IntervaloGiro`)))
  (`self.K2_AddActorLocalRotation` (`self.VelocidadRotacion`))
  (goto _label))

(fn `UserConstructionScript`)